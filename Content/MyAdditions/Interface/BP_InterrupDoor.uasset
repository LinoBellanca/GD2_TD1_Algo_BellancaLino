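; Pressure-plate style switch that activates linked objects, likely doors, when the third-person character enters its box with FirstToggle set.
; The overlap plays a sound at the stored PlateLocation, then sends ActivateMessage to each BPControllables entry implementing BPI_ControlInt.
; Each message also calls OpenClose, which re-captures the plate's relative location and restarts a timeline that offsets the plate from it.
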(event OnComponentBeginOverlap(Box)
  (params (OverlappedComponent :type Primitive%20Component%20Object%20Reference) (OtherActor :type Actor%20Object%20Reference) (OtherComp :type Primitive%20Component%20Object%20Reference) (OtherBodyIndex :type Integer) (bFromSweep :type Boolean) (SweepResult :type Hit%20Result%20Structure%20%28by%20ref%29))
  (bind _asbp_third_person_character (Utilities|Casting|CastToBP_ThirdPersonCharacter OtherActor))
  (if (Variables|/Game/ThirdPerson/Blueprints/BP_ThirdPersonCharacter.BP_ThirdPersonCharacter_C|GetFirstToggle _asbp_third_person_character)
    (Audio|PlaySoundatLocation "/Game/MyAdditions/Sounds/Interruptors/SC_InterActiv.SC_InterActiv" (Variables|Default|GetPlateLocation) "0, 0, 0" 1.0 1.0 0.0 0 0 0 0)
    (for _array_element (Variables|Default|GetBP_Controllables)
      (if (Utilities|DoesObjectImplementInterface _array_element "/Game/MyAdditions/Interface/BPI_ControlInt.BPI_ControlInt_C")
        (Class|BPIControlInt|Activate(Message) _array_element)
        (CallFunction|OpenClose)))))

(event Custom|OpenClose
  (Variables|Default|SetPlateLocation (Variables|/Script/Engine.SceneComponent|GetRelativeLocation (Variables|Default|GetPlate)))
  (bind _newtrack_0 (Timeline|PlateTimeline PlayFromStart)
    (:Update
      (Transformation|SetRelativeLocation (Variables|Default|GetPlate) (+ _newtrack_0 (Variables|Default|GetPlateLocation)) false false))))

(event EventBeginPlay)

(event Collision|EventActorBeginOverlap
  (params (OtherActor :type Actor%20Object%20Reference)))

(event EventTick
  (params (DeltaSeconds :type Float%20%28single-precision%29)))

(fn ConstructionScript)