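; BP_Door is a toggleable door that opens or closes on Activate and animates open at BeginPlay if IsOpen is set.
; ToggleDoor flips the PointLight and IsOpen, runs the matching event and, unless FirstDoor is set, sends add or remove messages to Light.
; Open and close timelines offset the Door's relative location from DoorLocation, triggering the door sound on every update.
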(event Custom|DoorClosing
  (Variables|Default|SetDoorLocation (Variables|Default|GetDoorLocation))
  (bind _newtrack_0 (Timeline|CloseTimeline PlayFromStart)
    (:Update
      (Transformation|SetRelativeLocation (Variables|Default|GetDoor) (+ _newtrack_0 (Variables|Default|GetDoorLocation)) false false)
      (Audio|PlaySoundatLocation "/Game/MyAdditions/Sounds/Doors/SC_DoorClose.SC_DoorClose" (Variables|Default|GetDoorLocation) "0, 0, 0" 1.0 1.0 0.0 0 0 0 0))))

(event Custom|DoorOpening
  (Variables|Default|SetDoorLocation (Variables|Default|GetDoorLocation))
  (bind _newtrack_0 (Timeline|OpenTimeline PlayFromStart)
    (:Update
      (Transformation|SetRelativeLocation (Variables|Default|GetDoor) (+ _newtrack_0 (Variables|Default|GetDoorLocation)) false false)
      (Audio|PlaySoundatLocation "/Game/MyAdditions/Sounds/Doors/SC_Door_Open.SC_Door_Open" (Variables|Default|GetDoorLocation) "0, 0, 0" 1.0 1.0 0.0 0 0 0 0))))

(event EventBeginPlay
  (if (Variables|Default|GetIsOpen)
    (CallFunction|DoorOpening)))

(event Collision|EventActorBeginOverlap
  (params (OtherActor :type Actor%20Object%20Reference)))

(event EventTick
  (params (DeltaSeconds :type Float%20%28single-precision%29)))

(event EventActivate
  (CallFunction|ToggleDoor))

(fn ConstructionScript)

(fn ToggleDoor
  (Rendering|SetVisibility (Variables|Default|GetPointLight) (not (Variables|/Script/Engine.SceneComponent|GetbVisible (Variables|Default|GetPointLight))) false)
  (if (Variables|Default|GetIsOpen)
    (CallFunction|DoorClosing)
    (Variables|Default|SetIsOpen false)
    (if (not (Variables|Default|GetFirstDoor))
      (Class|BPIControlInt|DoorRemover(Message) (Variables|Default|GetLight)))
    (else
      (CallFunction|DoorOpening)
      (Variables|Default|SetIsOpen true)
      (if (not (Variables|Default|GetFirstDoor))
        (Class|BPIControlInt|DoorAdder(Message) (Variables|Default|GetLight))))))