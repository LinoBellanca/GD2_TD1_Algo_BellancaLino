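; Light actor that cuts out on activation and comes back once its count of doors left to close reaches zero.
; Activate plays the off sound, toggles the spotlight and sets the counter to two.
; DoorAdder and DoorRemover adjust the counter and retry turn-on after short delays.
; At zero, turn-on destroys all BP_InterrupDoor actors, plays the on sound, calls CallActivateTolio and toggles the spotlight back.
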(event Custom|TurnLight
  (Utilities|FlowControl|FlipFlop))

(event EventBeginPlay)

(event Collision|EventActorBeginOverlap
  (params (OtherActor :type Actor%20Object%20Reference)))

(event EventTick
  (params (DeltaSeconds :type Float%20%28single-precision%29)))

(event EventTurnLighton
  (Utilities|FlowControl|Delay 0.5)
  (if (== (Variables|Default|GetDoorsToClose) 0)
    (bind _outactors (Actor|GetAllActorsOfClass "/Game/MyAdditions/Interface/BP_InterrupDoor.BP_InterrupDoor_C"))
    (Actor|DestroyActor _outactors)
    (Utilities|FlowControl|Delay 0.5)
    (Audio|PlaySoundatLocation "/Game/MyAdditions/Sounds/Light/SC_LightOn.SC_LightOn" (Transformation|GetWorldLocation (Variables|Default|GetLamp)) "0, 0, 0" 1.0 1.0 0.0 0 0 0 0)
    (Default|CallActivateTolio)
    (CallFunction|ToggleLight)))

(event EventActivate
  (Utilities|FlowControl|Delay 1.0)
  (Audio|PlaySoundatLocation "/Game/MyAdditions/Sounds/Light/SC_LightOff.SC_LightOff" (Transformation|GetWorldLocation (Variables|Default|GetLamp)) "0, 0, 0" 1.0 1.0 0.0 0 0 0 0)
  (CallFunction|ToggleLight)
  (Variables|Default|SetDoorsToClose 2))

(event EventDoorRemover
  ;[1 1 1] Compte le nombre de portes qu'il reste à fermer puis essaye d'allumer
  (CallFunction|RemoveDoor)
  (CallFunction|TurnLighton))

(event EventDoorAdder
  ;[1 1 1] Compte le nombre de portes qu'il reste à fermer puis essaye d'allumer
  (CallFunction|AddDoor)
  (CallFunction|TurnLighton))

(fn ConstructionScript)

(fn ToggleLight
  (bind _spotlight (Variables|Default|GetSpotLight))
  (Rendering|SetVisibility _spotlight (not (Variables|/Script/Engine.SceneComponent|GetbVisible _spotlight)) false))

(fn AddDoor
  (bind _result (Math|Integer|IncrementInt (Variables|Default|GetDoorsToClose))
    (:%20%20
      (Variables|Default|SetDoorsToClose _result))))

(fn RemoveDoor
  (bind _result (Math|Integer|DecrementInt (Variables|Default|GetDoorsToClose))
    (:%20%20
      (Variables|Default|SetDoorsToClose _result))))