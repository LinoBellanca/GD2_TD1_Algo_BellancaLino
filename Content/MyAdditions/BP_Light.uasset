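; BP_Light is a light actor that can be switched on and off through its PointLight component.
; TurnLight uses a FlipFlop to alternate the light's intensity between full and zero, recording the state in IsOn.
; Activate and Deactivate both call ToggleLight, which inverts component visibility, so either event toggles rather than setting a fixed state.
; The visibility path is independent of IsOn and intensity.
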(event Custom|TurnLight
  (Utilities|FlowControl|FlipFlop
    (:A
      (Variables|Default|SetIsOn true)
      (Rendering|Components|Light|SetIntensity (Variables|Default|GetPointLight) 1e+04))
    (:B
      (Variables|Default|SetIsOn false)
      (Rendering|Components|Light|SetIntensity (Variables|Default|GetPointLight) 0.0))))

(event EventBeginPlay)

(event Collision|EventActorBeginOverlap
  (params (OtherActor :type Actor%20Object%20Reference)))

(event EventTick
  (params (DeltaSeconds :type Float%20%28single-precision%29)))

(event EventDeactivate
  (CallFunction|ToggleLight))

(event EventActivate
  (CallFunction|ToggleLight))

(fn ConstructionScript)

(fn ToggleLight
  (bind _pointlight (Variables|Default|GetPointLight))
  (Rendering|SetVisibility _pointlight (not (Variables|/Script/Engine.SceneComponent|GetbVisible _pointlight)) false))