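; BP_Rashp is an NPC that stays idle until activated, then walks to a goal and chases the player.
; On BeginPlay it binds GoForward to the EventLauncher's activation event, which starts a slow AI move to the first GoalRef actor.
; Reaching the goal triggers ChasePlayer, which raises walk speed and moves toward the BP_ThirdPersonCharacter found by class lookup.
; A failed goal move only prints a debug string.
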(event Custom|GoForward
  (Variables|/Script/Engine.CharacterMovementComponent|SetMaxWalkSpeed (Variables|Character|GetCharacterMovement) 1e+02)
  (AI|AIMoveTo self "0.000000,0.000000,0.000000" (Utilities|Array|Get(acopy) (Variables|Default|GetGoalRef)) 5.0 false
    (:OnSuccess
      (CallFunction|ChasePlayer))
    (:OnFail
      (Development|PrintString "Hello"))))

(event Custom|ChasePlayer
  (Variables|/Script/Engine.CharacterMovementComponent|SetMaxWalkSpeed (Variables|Character|GetCharacterMovement) 4e+02)
  (bind _returnvalue (Actor|GetActorOfClass "/Game/ThirdPerson/Blueprints/BP_ThirdPersonCharacter.BP_ThirdPersonCharacter_C"))
  (AI|AIMoveTo self "0, 0, 0" _returnvalue 5.0 false))

(event EventBeginPlay
  (EventDispatchers|BindEventtoActivateRashp (Variables|Default|GetEventLauncher) (delegate Custom|GoForward)))

(event Collision|EventActorBeginOverlap
  (params (OtherActor :type Actor%20Object%20Reference)))

(event EventTick
  (params (DeltaSeconds :type Float%20%28single-precision%29)))

(fn ConstructionScript)