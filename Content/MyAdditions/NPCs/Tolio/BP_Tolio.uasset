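; BP_Tolio is an NPC that keeps turning toward the player and can send the game to the win level.
; FacePlayer re-runs itself through a tiny Delay instead of Tick, interpolating yaw toward the third-person character.
; BeginPlay also binds to EventLauncher's ActivateTolio event, which teleports Tolio to the BP_TolioGoal actor.
; A separate EforWin event opens Map_Win.
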(event Custom|FacePlayer
  (bind _returnvalue (Actor|GetActorOfClass "/Game/ThirdPerson/Blueprints/BP_ThirdPersonCharacter.BP_ThirdPersonCharacter_C"))
  (Transformation|SetActorRotation (Math|Rotator|MakeRotator 0.0 0.0 (.yaw (Class|KismetMathLibrary|RInterptoConstant (Transformation|GetActorRotation) (Math|Interpolation|RInterpTo (Math|Rotator|FindLookatRotation (Transformation|GetActorLocation) (Transformation|GetActorLocation _returnvalue)) "0, 0, 0" 0.0 0.0) (Utilities|Time|GetWorldDeltaSeconds) 1e+02))))
  (Utilities|FlowControl|Delay 0.001)
  (CallFunction|FacePlayer))

(event Custom|TPTolio
  (bind _returnvalue (Actor|GetActorOfClass "/Game/MyAdditions/NPCs/Tolio/BP_TolioGoal.BP_TolioGoal_C"))
  (Transformation|Teleport self (Transformation|GetActorLocation _returnvalue) "0, 0, 0"))

(event EventBeginPlay
  (CallFunction|FacePlayer)
  (EventDispatchers|BindEventtoActivateTolio (Variables|Default|GetEventLauncher) (delegate Custom|TPTolio)))

(event Collision|EventActorBeginOverlap
  (params (OtherActor :type Actor%20Object%20Reference)))

(event EventTick
  (params (DeltaSeconds :type Float%20%28single-precision%29)))

(event EventEforWin
  (Game|OpenLevel(byName) "Map_Win"))

(fn ConstructionScript)